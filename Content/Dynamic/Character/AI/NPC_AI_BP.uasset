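; AI controller for guard NPCs that runs the guard behavior tree and reacts to perception updates.
; BeginPlay sets up the blackboard with the player pawn as the initial enemy, then starts the tree.
; Sensing an actor without the "Enemy" tag stores it as the enemy and turns on the guard's aiming and firing animation flags.
; Losing it records the stored enemy's location as last seen, clears the key and resets those flags.
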(event OnTargetPerceptionUpdated(AIPerception)
  (params (Actor :type Actor%20Object%20Reference) (Stimulus :type AI%20Stimulus%20Structure))
  (bind _returnvalue (Pawn|GetControlledPawn))
  (if (not (Actor|ActorHasTag Actor "Enemy"))
    (if (.bSuccessfullySensed (Utilities|Struct|BreakAIStimulus Stimulus))
      (AI|Components|Blackboard|SetValueasObject (Variables|Default|GetBehaviorTree) (Variables|Default|GetEnemyKey) Actor) ; Set enemy in blackboard
      ;[1 1 1] Set boolean in UE4 character (i.e. the guard) used for animation states
      (bind _ascharacter_bp (Utilities|Casting|CastToCharacter_BP _returnvalue))
      (Variables|/Game/Dynamic/Character/Behavior/Character_BP.Character_BP_C|SetAiming _ascharacter_bp true)
      (Variables|/Game/Dynamic/Character/Behavior/Character_BP.Character_BP_C|SetFiring _ascharacter_bp true)
      (else
        (bind _asactor (Utilities|Casting|CastToActor (AI|Components|Blackboard|GetValueasObject (Variables|Default|GetBehaviorTree) (Variables|Default|GetEnemyKey))))
        (AI|Components|Blackboard|SetValueasVector (Variables|Default|GetBehaviorTree) (Variables|Default|GetLastSeenLocation) (Transformation|GetActorLocation _asactor)) ; Set location in blackboard
        (AI|Components|Blackboard|ClearValue (Variables|Default|GetBehaviorTree) (Variables|Default|GetEnemyKey)) ; Clear player value in blackboard (lost line of sight)
        (bind _ascharacter_bp_2 (Utilities|Casting|CastToCharacter_BP _returnvalue))
        (Variables|/Game/Dynamic/Character/Behavior/Character_BP.Character_BP_C|SetAiming _ascharacter_bp_2 false)
        (Variables|/Game/Dynamic/Character/Behavior/Character_BP.Character_BP_C|SetFiring _ascharacter_bp_2 false)))))

(event EventBeginPlay
  (bind _blackboardcomponent (Class|AIController|UseBlackboard "/Game/Dynamic/Character/AI/GuardBehaviorData.GuardBehaviorData"))
  (AI|Components|Blackboard|SetValueasObject _blackboardcomponent (Variables|Default|GetEnemyKey) (Game|Player|GetPlayerPawn 0))
  (AI|RunBehaviorTree "/Game/Dynamic/Character/AI/GuardBehavior.GuardBehavior")
  (Variables|Default|SetBehaviorTree _blackboardcomponent))

(fn ConstructionScript)