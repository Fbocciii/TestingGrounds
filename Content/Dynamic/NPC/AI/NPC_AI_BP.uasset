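; AI controller for guard NPCs that runs the GuardBehavior tree on the GuardBehaviorData blackboard.
; BeginPlay seeds EnemyKey with the player pawn and caches the blackboard in a variable named BehaviorTree.
; AI Perception sets EnemyKey to any sensed actor not tagged "Enemy".
; When such an actor is lost, it saves the stored enemy's location to LastSeenLocation and clears EnemyKey.
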(event OnTargetPerceptionUpdated(AIPerception)
  (params (Actor :type Actor%20Object%20Reference) (Stimulus :type AI%20Stimulus%20Structure))
  (if (not (Actor|ActorHasTag Actor "Enemy"))
    (if (.bSuccessfullySensed (Utilities|Struct|BreakAIStimulus Stimulus))
      (AI|Components|Blackboard|SetValueasObject (Variables|Default|GetBehaviorTree) (Variables|Default|GetEnemyKey) Actor)
      (else
        (bind _asactor (Utilities|Casting|CastToActor (AI|Components|Blackboard|GetValueasObject (Variables|Default|GetBehaviorTree) (Variables|Default|GetEnemyKey))))
        (AI|Components|Blackboard|SetValueasVector (Variables|Default|GetBehaviorTree) (Variables|Default|GetLastSeenLocation) (Transformation|GetActorLocation _asactor))
        (AI|Components|Blackboard|ClearValue (Variables|Default|GetBehaviorTree) (Variables|Default|GetEnemyKey))))))

(event EventBeginPlay
  (bind _blackboardcomponent (Class|AIController|UseBlackboard "/Game/Dynamic/NPC/AI/GuardBehaviorData.GuardBehaviorData"))
  (AI|Components|Blackboard|SetValueasObject _blackboardcomponent (Variables|Default|GetEnemyKey) (Game|Player|GetPlayerPawn 0))
  (AI|RunBehaviorTree "/Game/Dynamic/NPC/AI/GuardBehavior.GuardBehavior")
  (Variables|Default|SetBehaviorTree _blackboardcomponent))

(fn ConstructionScript)